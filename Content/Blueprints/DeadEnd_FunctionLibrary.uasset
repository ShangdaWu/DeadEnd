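; Blueprint function library that writes player gold, diamonds and the stats of characters A, B and C to the DeadEnd_SaveGame in slot "DeadEndSlot".
; Each update loads the slot, sets a field and saves at once, doing nothing if no save exists.
; The character updates repeat that load and save separately for every stat through a Sequence.
; GetSaveGameReference returns the loaded save object.
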(fn `GetSaveGameReference`
  (returns (`AsDead End Save Game` :type "/Game/Blueprints/DeadEnd_SaveGame Object Reference"))
  ;[1 1 1] 得到Savegame的引用
  (bind _returnvalue (`GameplayStatics.DoesSaveGameExist` "DeadEndSlot"))
  (if _returnvalue
    (bind _returnvalue_2 (`GameplayStatics.LoadGameFromSlot` "DeadEndSlot"))
    (bind _asdead_end_save_game (cast `/Game/Blueprints/DeadEnd_SaveGame` _returnvalue_2)
      (:`then`
        _)
      (:`CastFailed`
        _)))
  (return _asdead_end_save_game))

(fn `Update_Character_A_Data`
  (params (Character_A_Lv_Number :type Integer) (Character_A_Experience_Number :type Integer) (Character_A_NextExperience_Number :type Integer) (Character_A_Life_Number :type Integer) (Character_A_LifeRecovery_Number :type "Float (double-precision)") (Character_A_Stamina_Number :type Integer) (Character_A_StaminaRecovery_Number :type "Float (double-precision)") (Character_A_Lucky_Number :type Integer))
  ;[1 1 1] 循环检测角色A的等级
  (`|ExecutionSequence`
    (:`then_0`
      (bind _returnvalue (`GameplayStatics.DoesSaveGameExist` "DeadEndSlot"))
      (if _returnvalue
        (bind _returnvalue_2 (`GameplayStatics.LoadGameFromSlot` "DeadEndSlot"))
        (bind _asdead_end_save_game (cast `/Game/Blueprints/DeadEnd_SaveGame` _returnvalue_2))
        (set `/Game/Blueprints/DeadEnd_SaveGame.Character_A_Lv` Character_A_Lv_Number _asdead_end_save_game)
        (`GameplayStatics.SaveGameToSlot` _returnvalue_2 "DeadEndSlot")))
    (:`then_1`
      ;;[1 1 1] 循环检测角色A的当前经验值
      (bind _returnvalue_3 (`GameplayStatics.DoesSaveGameExist` "DeadEndSlot"))
      (if _returnvalue_3
        (bind _returnvalue_4 (`GameplayStatics.LoadGameFromSlot` "DeadEndSlot"))
        (bind _asdead_end_save_game_2 (cast `/Game/Blueprints/DeadEnd_SaveGame` _returnvalue_4))
        (set `/Game/Blueprints/DeadEnd_SaveGame.Character_A_Experience` Character_A_Experience_Number _asdead_end_save_game_2)
        (`GameplayStatics.SaveGameToSlot` _returnvalue_4 "DeadEndSlot")))
    (:`then_2`
      ;;[1 1 1] 循环检测角色A的下一级经验值
      (bind _returnvalue_5 (`GameplayStatics.DoesSaveGameExist` "DeadEndSlot"))
      (if _returnvalue_5
        (bind _returnvalue_6 (`GameplayStatics.LoadGameFromSlot` "DeadEndSlot"))
        (bind _asdead_end_save_game_3 (cast `/Game/Blueprints/DeadEnd_SaveGame` _returnvalue_6))
        (set `/Game/Blueprints/DeadEnd_SaveGame.Character_A_NextExperience` Character_A_NextExperience_Number _asdead_end_save_game_3)
        (`GameplayStatics.SaveGameToSlot` _returnvalue_6 "DeadEndSlot")))
    (:`then_3`
      ;;[1 1 1] 循环检测角色A的当前生命值
      (bind _returnvalue_7 (`GameplayStatics.DoesSaveGameExist` "DeadEndSlot"))
      (if _returnvalue_7
        (bind _returnvalue_8 (`GameplayStatics.LoadGameFromSlot` "DeadEndSlot"))
        (bind _asdead_end_save_game_4 (cast `/Game/Blueprints/DeadEnd_SaveGame` _returnvalue_8))
        (set `/Game/Blueprints/DeadEnd_SaveGame.Character_A_Life` Character_A_Life_Number _asdead_end_save_game_4)
        (`GameplayStatics.SaveGameToSlot` _returnvalue_8 "DeadEndSlot")))
    (:`then_4`
      ;;[1 1 1] 循环检测角色A的当前生命恢复值
      (bind _returnvalue_9 (`GameplayStatics.DoesSaveGameExist` "DeadEndSlot"))
      (if _returnvalue_9
        (bind _returnvalue_10 (`GameplayStatics.LoadGameFromSlot` "DeadEndSlot"))
        (bind _asdead_end_save_game_5 (cast `/Game/Blueprints/DeadEnd_SaveGame` _returnvalue_10))
        (set `/Game/Blueprints/DeadEnd_SaveGame.Character_A_LifeRecovery` Character_A_LifeRecovery_Number _asdead_end_save_game_5)
        (`GameplayStatics.SaveGameToSlot` _returnvalue_10 "DeadEndSlot")))
    (:`then_5`
      ;;[1 1 1] 循环检测角色A的当前耐力值
      (bind _returnvalue_11 (`GameplayStatics.DoesSaveGameExist` "DeadEndSlot"))
      (if _returnvalue_11
        (bind _returnvalue_12 (`GameplayStatics.LoadGameFromSlot` "DeadEndSlot"))
        (bind _asdead_end_save_game_6 (cast `/Game/Blueprints/DeadEnd_SaveGame` _returnvalue_12))
        (set `/Game/Blueprints/DeadEnd_SaveGame.Character_A_Stamina` Character_A_Stamina_Number _asdead_end_save_game_6)
        (`GameplayStatics.SaveGameToSlot` _returnvalue_12 "DeadEndSlot")))
    (:`then_6`
      ;;[1 1 1] 循环检测角色A的当前耐力恢复值
      (bind _returnvalue_13 (`GameplayStatics.DoesSaveGameExist` "DeadEndSlot"))
      (if _returnvalue_13
        (bind _returnvalue_14 (`GameplayStatics.LoadGameFromSlot` "DeadEndSlot"))
        (bind _asdead_end_save_game_7 (cast `/Game/Blueprints/DeadEnd_SaveGame` _returnvalue_14))
        (set `/Game/Blueprints/DeadEnd_SaveGame.Character_A_StaminaRecovery` Character_A_StaminaRecovery_Number _asdead_end_save_game_7)
        (`GameplayStatics.SaveGameToSlot` _returnvalue_14 "DeadEndSlot")))
    (:`then_7`
      ;;[1 1 1] 循环检测角色A的当前幸运值
      (bind _returnvalue_15 (`GameplayStatics.DoesSaveGameExist` "DeadEndSlot"))
      (if _returnvalue_15
        (bind _returnvalue_16 (`GameplayStatics.LoadGameFromSlot` "DeadEndSlot"))
        (bind _asdead_end_save_game_8 (cast `/Game/Blueprints/DeadEnd_SaveGame` _returnvalue_16))
        (set `/Game/Blueprints/DeadEnd_SaveGame.Character_A_Lucky` Character_A_Lucky_Number _asdead_end_save_game_8)
        (`GameplayStatics.SaveGameToSlot` _returnvalue_16 "DeadEndSlot")))))

(fn `Update_Character_B_Data`
  (params (Character_B_Lv_Nmuber :type Integer) (Character_B_Experience_Number :type Integer) (Character_B_NextExperience_Number :type Integer) (Character_B_Life_Number :type Integer) (Character_B_LifeRecovery_Number :type "Float (double-precision)") (Character_B_Stamina_Number :type Integer) (Character_B_StaminaRecovery_Number :type "Float (double-precision)") (Character_B_Lucky_Numberram :type Integer))
  ;[1 1 1] 循环检测角色B的等级
  (`|ExecutionSequence`
    (:`then_0`
      (bind _returnvalue (`GameplayStatics.DoesSaveGameExist` "DeadEndSlot"))
      (if _returnvalue
        (bind _returnvalue_2 (`GameplayStatics.LoadGameFromSlot` "DeadEndSlot"))
        (bind _asdead_end_save_game (cast `/Game/Blueprints/DeadEnd_SaveGame` _returnvalue_2))
        (set `/Game/Blueprints/DeadEnd_SaveGame.Character_B_Lv` Character_B_Lv_Nmuber _asdead_end_save_game)
        (`GameplayStatics.SaveGameToSlot` _returnvalue_2 "DeadEndSlot")))
    (:`then_1`
      ;;[1 1 1] 循环检测角色B的当前经验值
      (bind _returnvalue_3 (`GameplayStatics.DoesSaveGameExist` "DeadEndSlot"))
      (if _returnvalue_3
        (bind _returnvalue_4 (`GameplayStatics.LoadGameFromSlot` "DeadEndSlot"))
        (bind _asdead_end_save_game_2 (cast `/Game/Blueprints/DeadEnd_SaveGame` _returnvalue_4))
        (set `/Game/Blueprints/DeadEnd_SaveGame.Character_B_Experience` Character_B_Experience_Number _asdead_end_save_game_2)
        (`GameplayStatics.SaveGameToSlot` _returnvalue_4 "DeadEndSlot")))
    (:`then_2`
      ;;[1 1 1] 循环检测角色B的下一级经验值
      (bind _returnvalue_5 (`GameplayStatics.DoesSaveGameExist` "DeadEndSlot"))
      (if _returnvalue_5
        (bind _returnvalue_6 (`GameplayStatics.LoadGameFromSlot` "DeadEndSlot"))
        (bind _asdead_end_save_game_3 (cast `/Game/Blueprints/DeadEnd_SaveGame` _returnvalue_6))
        (set `/Game/Blueprints/DeadEnd_SaveGame.Character_B_NextExperience` Character_B_NextExperience_Number _asdead_end_save_game_3)
        (`GameplayStatics.SaveGameToSlot` _returnvalue_6 "DeadEndSlot")))
    (:`then_3`
      ;;[1 1 1] 循环检测角色B的当前生命值
      (bind _returnvalue_7 (`GameplayStatics.DoesSaveGameExist` "DeadEndSlot"))
      (if _returnvalue_7
        (bind _returnvalue_8 (`GameplayStatics.LoadGameFromSlot` "DeadEndSlot"))
        (bind _asdead_end_save_game_4 (cast `/Game/Blueprints/DeadEnd_SaveGame` _returnvalue_8))
        (set `/Game/Blueprints/DeadEnd_SaveGame.Character_B_Life` Character_B_Life_Number _asdead_end_save_game_4)
        (`GameplayStatics.SaveGameToSlot` _returnvalue_8 "DeadEndSlot")))
    (:`then_4`
      ;;[1 1 1] 循环检测角色B的当前生命恢复值
      (bind _returnvalue_9 (`GameplayStatics.DoesSaveGameExist` "DeadEndSlot"))
      (if _returnvalue_9
        (bind _returnvalue_10 (`GameplayStatics.LoadGameFromSlot` "DeadEndSlot"))
        (bind _asdead_end_save_game_5 (cast `/Game/Blueprints/DeadEnd_SaveGame` _returnvalue_10))
        (set `/Game/Blueprints/DeadEnd_SaveGame.Character_B_LifeRecovery` Character_B_LifeRecovery_Number _asdead_end_save_game_5)
        (`GameplayStatics.SaveGameToSlot` _returnvalue_10 "DeadEndSlot")))
    (:`then_5`
      ;;[1 1 1] 循环检测角色B的当前耐力值
      (bind _returnvalue_11 (`GameplayStatics.DoesSaveGameExist` "DeadEndSlot"))
      (if _returnvalue_11
        (bind _returnvalue_12 (`GameplayStatics.LoadGameFromSlot` "DeadEndSlot"))
        (bind _asdead_end_save_game_6 (cast `/Game/Blueprints/DeadEnd_SaveGame` _returnvalue_12))
        (set `/Game/Blueprints/DeadEnd_SaveGame.Character_B_Stamina` Character_B_Stamina_Number _asdead_end_save_game_6)
        (`GameplayStatics.SaveGameToSlot` _returnvalue_12 "DeadEndSlot")))
    (:`then_6`
      ;;[1 1 1] 循环检测角色B的当前耐力恢复值
      (bind _returnvalue_13 (`GameplayStatics.DoesSaveGameExist` "DeadEndSlot"))
      (if _returnvalue_13
        (bind _returnvalue_14 (`GameplayStatics.LoadGameFromSlot` "DeadEndSlot"))
        (bind _asdead_end_save_game_7 (cast `/Game/Blueprints/DeadEnd_SaveGame` _returnvalue_14))
        (set `/Game/Blueprints/DeadEnd_SaveGame.Character_B_StaminaRecovery` Character_B_StaminaRecovery_Number _asdead_end_save_game_7)
        (`GameplayStatics.SaveGameToSlot` _returnvalue_14 "DeadEndSlot")))
    (:`then_7`
      ;;[1 1 1] 循环检测角色B的当前幸运值
      (bind _returnvalue_15 (`GameplayStatics.DoesSaveGameExist` "DeadEndSlot"))
      (if _returnvalue_15
        (bind _returnvalue_16 (`GameplayStatics.LoadGameFromSlot` "DeadEndSlot"))
        (bind _asdead_end_save_game_8 (cast `/Game/Blueprints/DeadEnd_SaveGame` _returnvalue_16))
        (set `/Game/Blueprints/DeadEnd_SaveGame.Character_B_Lucky` Character_B_Lucky_Numberram _asdead_end_save_game_8)
        (`GameplayStatics.SaveGameToSlot` _returnvalue_16 "DeadEndSlot")))))

(fn `Update_Character_C_Data`
  (params (Character_C_Lv_Nmuber :type Integer) (Character_C_Experience_Number :type Integer) (Character_C_NextExperience_Number :type Integer) (Character_C_Life_Number :type Integer) (Character_C_LifeRecovery_Number :type "Float (double-precision)") (Character_C_Stamina_Number :type Integer) (Character_C_StaminaRecovery_Number :type "Float (double-precision)") (Character_C_Lucky_Numberram :type Integer))
  ;[1 1 1] 循环检测角色C的等级
  (`|ExecutionSequence`
    (:`then_0`
      (bind _returnvalue (`GameplayStatics.DoesSaveGameExist` "DeadEndSlot"))
      (if _returnvalue
        (bind _returnvalue_2 (`GameplayStatics.LoadGameFromSlot` "DeadEndSlot"))
        (bind _asdead_end_save_game (cast `/Game/Blueprints/DeadEnd_SaveGame` _returnvalue_2))
        (set `/Game/Blueprints/DeadEnd_SaveGame.Character_C_Lv` Character_C_Lv_Nmuber _asdead_end_save_game)
        (`GameplayStatics.SaveGameToSlot` _returnvalue_2 "DeadEndSlot")))
    (:`then_1`
      ;;[1 1 1] 循环检测角色B的当前经验值
      (bind _returnvalue_3 (`GameplayStatics.DoesSaveGameExist` "DeadEndSlot"))
      (if _returnvalue_3
        (bind _returnvalue_4 (`GameplayStatics.LoadGameFromSlot` "DeadEndSlot"))
        (bind _asdead_end_save_game_2 (cast `/Game/Blueprints/DeadEnd_SaveGame` _returnvalue_4))
        (set `/Game/Blueprints/DeadEnd_SaveGame.Character_C_Experience` Character_C_Experience_Number _asdead_end_save_game_2)
        (`GameplayStatics.SaveGameToSlot` _returnvalue_4 "DeadEndSlot")))
    (:`then_2`
      ;;[1 1 1] 循环检测角色B的下一级经验值
      (bind _returnvalue_5 (`GameplayStatics.DoesSaveGameExist` "DeadEndSlot"))
      (if _returnvalue_5
        (bind _returnvalue_6 (`GameplayStatics.LoadGameFromSlot` "DeadEndSlot"))
        (bind _asdead_end_save_game_3 (cast `/Game/Blueprints/DeadEnd_SaveGame` _returnvalue_6))
        (set `/Game/Blueprints/DeadEnd_SaveGame.Character_C_NextExperience` Character_C_NextExperience_Number _asdead_end_save_game_3)
        (`GameplayStatics.SaveGameToSlot` _returnvalue_6 "DeadEndSlot")))
    (:`then_3`
      ;;[1 1 1] 循环检测角色B的当前生命值
      (bind _returnvalue_7 (`GameplayStatics.DoesSaveGameExist` "DeadEndSlot"))
      (if _returnvalue_7
        (bind _returnvalue_8 (`GameplayStatics.LoadGameFromSlot` "DeadEndSlot"))
        (bind _asdead_end_save_game_4 (cast `/Game/Blueprints/DeadEnd_SaveGame` _returnvalue_8))
        (set `/Game/Blueprints/DeadEnd_SaveGame.Character_C_Life` Character_C_Life_Number _asdead_end_save_game_4)
        (`GameplayStatics.SaveGameToSlot` _returnvalue_8 "DeadEndSlot")))
    (:`then_4`
      ;;[1 1 1] 循环检测角色B的当前生命恢复值
      (bind _returnvalue_9 (`GameplayStatics.DoesSaveGameExist` "DeadEndSlot"))
      (if _returnvalue_9
        (bind _returnvalue_10 (`GameplayStatics.LoadGameFromSlot` "DeadEndSlot"))
        (bind _asdead_end_save_game_5 (cast `/Game/Blueprints/DeadEnd_SaveGame` _returnvalue_10))
        (set `/Game/Blueprints/DeadEnd_SaveGame.Character_C_LifeRecovery` Character_C_LifeRecovery_Number _asdead_end_save_game_5)
        (`GameplayStatics.SaveGameToSlot` _returnvalue_10 "DeadEndSlot")))
    (:`then_5`
      ;;[1 1 1] 循环检测角色B的当前耐力值
      (bind _returnvalue_11 (`GameplayStatics.DoesSaveGameExist` "DeadEndSlot"))
      (if _returnvalue_11
        (bind _returnvalue_12 (`GameplayStatics.LoadGameFromSlot` "DeadEndSlot"))
        (bind _asdead_end_save_game_6 (cast `/Game/Blueprints/DeadEnd_SaveGame` _returnvalue_12))
        (set `/Game/Blueprints/DeadEnd_SaveGame.Character_C_Stamina` Character_C_Stamina_Number _asdead_end_save_game_6)
        (`GameplayStatics.SaveGameToSlot` _returnvalue_12 "DeadEndSlot")))
    (:`then_6`
      ;;[1 1 1] 循环检测角色B的当前耐力恢复值
      (bind _returnvalue_13 (`GameplayStatics.DoesSaveGameExist` "DeadEndSlot"))
      (if _returnvalue_13
        (bind _returnvalue_14 (`GameplayStatics.LoadGameFromSlot` "DeadEndSlot"))
        (bind _asdead_end_save_game_7 (cast `/Game/Blueprints/DeadEnd_SaveGame` _returnvalue_14))
        (set `/Game/Blueprints/DeadEnd_SaveGame.Character_C_StaminaRecovery` Character_C_StaminaRecovery_Number _asdead_end_save_game_7)
        (`GameplayStatics.SaveGameToSlot` _returnvalue_14 "DeadEndSlot")))
    (:`then_7`
      ;;[1 1 1] 循环检测角色B的当前幸运值
      (bind _returnvalue_15 (`GameplayStatics.DoesSaveGameExist` "DeadEndSlot"))
      (if _returnvalue_15
        (bind _returnvalue_16 (`GameplayStatics.LoadGameFromSlot` "DeadEndSlot"))
        (bind _asdead_end_save_game_8 (cast `/Game/Blueprints/DeadEnd_SaveGame` _returnvalue_16))
        (set `/Game/Blueprints/DeadEnd_SaveGame.Character_C_Lucky` Character_C_Lucky_Numberram _asdead_end_save_game_8)
        (`GameplayStatics.SaveGameToSlot` _returnvalue_16 "DeadEndSlot")))))

(fn `Update_Diamond`
  (params (Diamond_Number :type Integer))
  ;[1 1 1] 循环检测钻石
  (bind _returnvalue (`GameplayStatics.DoesSaveGameExist` "DeadEndSlot"))
  (if _returnvalue
    (bind _returnvalue_2 (`GameplayStatics.LoadGameFromSlot` "DeadEndSlot"))
    (bind _asdead_end_save_game (cast `/Game/Blueprints/DeadEnd_SaveGame` _returnvalue_2))
    (set `/Game/Blueprints/DeadEnd_SaveGame.Player_Diamond` Diamond_Number _asdead_end_save_game)
    (`GameplayStatics.SaveGameToSlot` _returnvalue_2 "DeadEndSlot")))

(fn `Update_Gold`
  (params (Gold_Number :type Integer))
  ;[1 1 1] 循环检测金币
  (bind _returnvalue (`GameplayStatics.DoesSaveGameExist` "DeadEndSlot"))
  (if _returnvalue
    (bind _returnvalue_2 (`GameplayStatics.LoadGameFromSlot` "DeadEndSlot"))
    (bind _asdead_end_save_game (cast `/Game/Blueprints/DeadEnd_SaveGame` _returnvalue_2))
    (set `/Game/Blueprints/DeadEnd_SaveGame.Player_Gold` Gold_Number _asdead_end_save_game)
    (`GameplayStatics.SaveGameToSlot` _returnvalue_2 "DeadEndSlot")))