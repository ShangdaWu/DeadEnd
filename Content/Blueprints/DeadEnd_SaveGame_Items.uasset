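; DeadEnd_SaveGame_Items is, by its name, the Dead End save-game object for items, holding individually numbered item variables sorted into five color tiers.
; Its Items_Group event rebuilds the White, Green, Blue, Purple and Orange group arrays from those variables, using a separate ID range per color.
; The White group is twice the size of each other group, and the graph contains no save or load logic.
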(event `Items_Group`
  (set `self.Items_White_Group` (`|MakeArray` (`self.Items_10000`) (`self.Items_10001`) (`self.Items_10002`) (`self.Items_10003`) (`self.Items_10004`) (`self.Items_10005`) (`self.Items_10006`) (`self.Items_10007`) (`self.Items_10008`) (`self.Items_10009`) (`self.Items_10010`) (`self.Items_10011`) (`self.Items_10012`) (`self.Items_10013`) (`self.Items_10014`) (`self.Items_10015`) (`self.Items_10016`) (`self.Items_10017`) (`self.Items_10018`) (`self.Items_10019`) (`self.Items_10020`) (`self.Items_10021`) (`self.Items_10022`) (`self.Items_10023`) (`self.Items_10024`) (`self.Items_10025`) (`self.Items_10026`) (`self.Items_10027`)))
  (set `self.Items_Green_Group` (`|MakeArray` (`self.Items_20000`) (`self.Items_20001`) (`self.Items_20002`) (`self.Items_20003`) (`self.Items_20004`) (`self.Items_20005`) (`self.Items_20006`) (`self.Items_20007`) (`self.Items_20008`) (`self.Items_20009`) (`self.Items_20010`) (`self.Items_20011`) (`self.Items_20012`) (`self.Items_20013`)))
  (set `self.Items_Blue_Group` (`|MakeArray` (`self.Items_30000`) (`self.Items_30001`) (`self.Items_30002`) (`self.Items_30003`) (`self.Items_30004`) (`self.Items_30005`) (`self.Items_30006`) (`self.Items_30007`) (`self.Items_30008`) (`self.Items_30009`) (`self.Items_30010`) (`self.Items_30011`) (`self.Items_30012`) (`self.Items_30013`)))
  (set `self.Items_Purple_Group` (`|MakeArray` (`self.Items_40000`) (`self.Items_40001`) (`self.Items_40002`) (`self.Items_40003`) (`self.Items_40004`) (`self.Items_40005`) (`self.Items_40006`) (`self.Items_40007`) (`self.Items_40008`) (`self.Items_40009`) (`self.Items_40010`) (`self.Items_40011`) (`self.Items_40012`) (`self.Items_40013`)))
  (set `self.Items_Orange_Group` (`|MakeArray` (`self.Items_50000`) (`self.Items_50001`) (`self.Items_50002`) (`self.Items_50003`) (`self.Items_50004`) (`self.Items_50005`) (`self.Items_50006`) (`self.Items_50007`) (`self.Items_50008`) (`self.Items_50009`) (`self.Items_50010`) (`self.Items_50011`) (`self.Items_50012`) (`self.Items_50013`))))